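; BP_Wire01 is a construction-script spline tool that builds configurable wires from spline mesh components.
; SplineMeshVar places segments either between spline points or at Spacing intervals along the length, with tangents scaled by TangentScale.
; WireVar selects one of six component variants and whether one or two material slots are set.
; Each segment gets uniform WireSize scale and dynamic MI_Wire instances driven by color, dirt, specular, roughness and TextureVar texture sets.
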(fn `UserConstructionScript`
  (bind _conponent_1 (`self.Conponent 1`))
  (bind _spline (`self.Spline`))
  (bind _spline_2 (`self.Spline`))
  (bind _wire_size (`self.Wire Size`))
  (bind _points (`self.Points`))
  (bind _spacing (`self.Spacing`))
  (bind _tangent_scale (`self.Tangent Scale`))
  (bind _m1 (`self.M1`))
  (bind _m2 (`self.M2`))
  (bind (_location _tangent) (`SplineComponent.GetLocationAndTangentAtSplinePoint` _spline _points "Local"))
  (bind (_location_2 _tangent_2) (`SplineComponent.GetLocationAndTangentAtSplinePoint` _spline (+ _points 1) "Local"))
  (set `self.Conponent 1` null)
  (switch `int` (`self.Spline Mesh Var`)
    (:`Default`
      (for _index (range (+ (- (`SplineComponent.GetNumberOfSplinePoints` (`self.Spline`)) 2) 1)) :!label _label
        (set `self.Points` _index)
        (switch `int` (`self.Wire Var`)
          (:`Default`
            (bind _returnvalue (`AddComponent|NODE_AddSplineMeshComponent-0` :!label _label_2))
            (set `self.Conponent 1` _returnvalue))
          (:`0`
            (goto _label_2))
          (:`1`
            (bind _returnvalue_2 (`AddComponent|NODE_AddSplineMeshComponent-1`))
            (set `self.Conponent 1` _returnvalue_2))
          (:`2`
            (bind _returnvalue_3 (`AddComponent|NODE_AddSplineMeshComponent-2`))
            (set `self.Conponent 1` _returnvalue_3))
          (:`3`
            (bind _returnvalue_4 (`AddComponent|NODE_AddSplineMeshComponent-7`))
            (set `self.Conponent 1` _returnvalue_4))
          (:`4`
            (bind _returnvalue_5 (`AddComponent|NODE_AddSplineMeshComponent-8`))
            (set `self.Conponent 1` _returnvalue_5))
          (:`5`
            (bind _returnvalue_6 (`AddComponent|NODE_AddSplineMeshComponent-9`))
            (set `self.Conponent 1` _returnvalue_6)))
        (`SplineMeshComponent.SetStartAndEnd` _conponent_1 _location _tangent _location_2 _tangent_2 true)
        (`SplineMeshComponent.SetStartScale` _conponent_1 (`KismetMathLibrary.MakeVector2D` _wire_size _wire_size) true :!label _label_3)
        (`SplineMeshComponent.SetEndScale` _conponent_1 (`KismetMathLibrary.MakeVector2D` _wire_size _wire_size) true)
        (bind _returnvalue_7 (`KismetMaterialLibrary.CreateDynamicMaterialInstance` "/Game/ScienceLab/Materials/Blueprint/MI_Wire.MI_Wire"))
        (set `self.M1` _returnvalue_7)
        (bind _returnvalue_8 (`KismetMaterialLibrary.CreateDynamicMaterialInstance` "/Game/ScienceLab/Materials/Blueprint/MI_Wire.MI_Wire"))
        (set `self.M2` _returnvalue_8)
        (switch `int` (`self.Wire Var`)
          (:`Default`
            (`PrimitiveComponent.SetMaterial` _conponent_1 0 _m1 :!label _label_4))
          (:`0`
            (goto _label_4))
          (:`1`
            (goto _label_4))
          (:`2`
            (goto _label_4))
          (:`3`
            (`PrimitiveComponent.SetMaterial` _conponent_1 1 _m2 :!label _label_5)
            (`PrimitiveComponent.SetMaterial` _conponent_1 0 _m1))
          (:`4`
            (goto _label_5))
          (:`5`
            (goto _label_5)))
        (`MaterialInstanceDynamic.SetVectorParameterValue` _m1 "diffuse color" (`self.Color`))
        (`MaterialInstanceDynamic.SetScalarParameterValue` _m1 "spec" (`self.Specular`))
        (`MaterialInstanceDynamic.SetScalarParameterValue` _m2 "spec" (`self.Specular`))
        (`MaterialInstanceDynamic.SetScalarParameterValue` _m1 "Roughness" (`self.Roughness`))
        (`MaterialInstanceDynamic.SetScalarParameterValue` _m2 "Roughness" (`self.Roughness`))
        (`MaterialInstanceDynamic.SetVectorParameterValue` _m1 "additional diffuse color" (`self.Dirt Color`))
        (`MaterialInstanceDynamic.SetVectorParameterValue` _m2 "additional diffuse color" (`self.Dirt Color`))
        (`MaterialInstanceDynamic.SetVectorParameterValue` _m2 "diffuse color" (`self.Color2`))
        (switch `int` (`self.Texture var`)
          (:`Default`
            (`MaterialInstanceDynamic.SetTextureParameterValue` _m1 "Diffuse" "/Game/ScienceLab/Textures/BaseTextures/T_BW_D.T_BW_D" :!label _label_6)
            (`MaterialInstanceDynamic.SetTextureParameterValue` _m2 "Diffuse" "/Game/ScienceLab/Textures/BaseTextures/T_BW_D.T_BW_D")
            (`MaterialInstanceDynamic.SetTextureParameterValue` _m1 "Normal" "/Game/ScienceLab/Textures/BaseTextures/T_B_N.T_B_N")
            (`MaterialInstanceDynamic.SetTextureParameterValue` _m2 "Normal" "/Game/ScienceLab/Textures/BaseTextures/T_B_N.T_B_N")
            (`MaterialInstanceDynamic.SetTextureParameterValue` _m1 "SRMH" "/Game/ScienceLab/Textures/BaseTextures/T_BG_D.T_BG_D")
            (`MaterialInstanceDynamic.SetTextureParameterValue` _m2 "SRMH" "/Game/ScienceLab/Textures/BaseTextures/T_BG_D.T_BG_D"))
          (:`0`
            (goto _label_6))
          (:`1`
            (`MaterialInstanceDynamic.SetTextureParameterValue` _m1 "Diffuse" "/Game/ScienceLab/Textures/Blueprint/T_Wire01_D.T_Wire01_D")
            (`MaterialInstanceDynamic.SetTextureParameterValue` _m1 "Normal" "/Game/ScienceLab/Textures/Blueprint/T_Wire01_N.T_Wire01_N")
            (`MaterialInstanceDynamic.SetTextureParameterValue` _m1 "SRMH" "/Game/ScienceLab/Textures/Blueprint/T_Wire01_SRM.T_Wire01_SRM"))
          (:`2`
            (`MaterialInstanceDynamic.SetTextureParameterValue` _m1 "Diffuse" "/Game/ScienceLab/Textures/Blueprint/T_Wire02_D.T_Wire02_D")
            (`MaterialInstanceDynamic.SetTextureParameterValue` _m1 "Normal" "/Game/ScienceLab/Textures/BaseTextures/T_B_N.T_B_N")
            (`MaterialInstanceDynamic.SetTextureParameterValue` _m1 "SRMH" "/Game/ScienceLab/Textures/BaseTextures/T_BG_D.T_BG_D")))))
    (:`0`
      (goto _label))
    (:`1`
      (for _index_2 (range (+ (`.ReturnValue` (`KismetMathLibrary.FMod` (`SplineComponent.GetSplineLength` _spline_2) _spacing)) 1))
        (switch `int` (`self.Wire Var`)
          (:`Default`
            (bind _returnvalue_9 (`AddComponent|NODE_AddSplineMeshComponent-4` :!label _label_7))
            (set `self.Conponent 1` _returnvalue_9))
          (:`0`
            (goto _label_7))
          (:`1`
            (bind _returnvalue_10 (`AddComponent|NODE_AddSplineMeshComponent-5`))
            (set `self.Conponent 1` _returnvalue_10))
          (:`2`
            (bind _returnvalue_11 (`AddComponent|NODE_AddSplineMeshComponent-6`))
            (set `self.Conponent 1` _returnvalue_11))
          (:`3`
            (bind _returnvalue_12 (`AddComponent|NODE_AddSplineMeshComponent-10`))
            (set `self.Conponent 1` _returnvalue_12))
          (:`4`
            (bind _returnvalue_13 (`AddComponent|NODE_AddSplineMeshComponent-11`))
            (set `self.Conponent 1` _returnvalue_13))
          (:`5`
            (bind _returnvalue_14 (`AddComponent|NODE_AddSplineMeshComponent-12`))
            (set `self.Conponent 1` _returnvalue_14)))
        (bind _returnvalue_15 (* _index_2 _spacing))
        (bind _returnvalue_16 (+ _returnvalue_15 _spacing))
        (`SplineMeshComponent.SetStartAndEnd` _conponent_1 (`SplineComponent.GetLocationAtDistanceAlongSpline` _spline_2 _returnvalue_15 "Local") (* (`SplineComponent.GetDirectionAtDistanceAlongSpline` _spline_2 _returnvalue_15 "Local") _tangent_scale) (`SplineComponent.GetLocationAtDistanceAlongSpline` _spline_2 _returnvalue_16 "Local") (* (`SplineComponent.GetDirectionAtDistanceAlongSpline` _spline_2 _returnvalue_16 "Local") _tangent_scale) true)
        (goto _label_3)))))